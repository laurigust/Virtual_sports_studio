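; BP_RB is the player card for the RB position in a lineup scene driven by Aximmetry inputs.
; BeginPlay creates dynamic materials for the name holder and photo.
; Every Tick feeds the RB photo video, name text and shared lineup color into them and the text component, with text size switching on whether the name is empty.
; PlayIO plays the IO sequence.
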(event `self.ReceiveBeginPlay`
  (bind _playerphoto (`self.PlayerPhoto`))
  (bind _playernameholder (`self.PlayerNameHolder`))
  (`|ExecutionSequence`
    (:`then_0`
      ;[1 1 1] Set Players card color
      (bind _returnvalue (`PrimitiveComponent.CreateDynamicMaterialInstance` _playernameholder 0 "/Game/Scena/Lineup/NameHolder.NameHolder" "None"))
      (`PrimitiveComponent.SetMaterial` _playernameholder 0 _returnvalue))
    (:`then_1`
      ;[1 1 1] Set player photo
      (bind _returnvalue_2 (`PrimitiveComponent.CreateDynamicMaterialInstance` _playerphoto 0 "/Game/Scena/Lineup/Player_texture.Player_texture" "None"))
      (`PrimitiveComponent.SetMaterial` _playerphoto 0 _returnvalue_2))))

(event `self.ReceiveTick`
  (params (DeltaSeconds :type "Float (single-precision)"))
  (bind _returnvalue (`self.GetAximmetryText` "RB_NAME"))
  (bind _playername (`self.PlayerName`))
  (`|ExecutionSequence`
    (:`then_0`
      ;[1 1 1] Set player photo
      (bind _returnvalue_2 (`self.GetAximmetryVideo` "RB_PHOTO"))
      (`MaterialInstanceDynamic.SetTextureParameterValue` (stale `self.ReceiveBeginPlay` _returnvalue_2) "PlayerTexture" _returnvalue_2))
    (:`then_1`
      ;[1 1 1] Controll player name font size
      (`TextRenderComponent.K2_SetText` _playername _returnvalue))
    (:`then_2`
      (if (> (`KismetStringLibrary.Len` (`KismetTextLibrary.Conv_TextToString` _returnvalue)) 0)
        (`TextRenderComponent.SetWorldSize` _playername 6.0)
        (else
          (`TextRenderComponent.SetWorldSize` _playername 7.0))))
    (:`then_3`
      ;[1 1 1] Set Players card color
      (`MaterialInstanceDynamic.SetVectorParameterValue` (stale `self.ReceiveBeginPlay` _returnvalue) "Color" (`self.GetAximmetryColor` "LINEUP COLOR")))))

(event `PlayIO`
  (`ActorSequenceComponent.PlaySequence` (`self.IO`)))

(fn `UserConstructionScript`)