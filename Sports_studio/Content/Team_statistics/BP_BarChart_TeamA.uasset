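; Animated 3D bar chart actor, apparently for Team A's match statistics, with a value label above each bar.
; Construction script creates meshes and labels from DataValues and binds configurable curves to the Grow and Fade timelines.
; BuildChart toggles between revealing (bars grow, then text fades in) and hiding in reverse.
; While animating, bars scale against the higher TeamH/TeamA value per Game_Statistics row and take curve-driven colors through dynamic materials.
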(event `self.BuildChart`
  (bind (_size_x _size_y) (`KismetMathLibrary.BreakVector2D` (`self.Size`)))
  (bind _defaultsceneroot (`self.DefaultSceneRoot`))
  (bind _initatzero (`self.InitAtZero`))
  (bind _isa (`/Engine/EditorBlueprintResources/StandardMacros.FlipFlop`)
    (:`A`
      (if _initatzero
        (`SceneComponent.SetVisibility` _defaultsceneroot true true :!label _label)
        (bind (_direction _growfactor) (`Timeline|GrowTimeline` :`NewTime` 1.0 :!via `PlayFromStart` :!label _label_2)
          (:`Update`
            ;[1 1 1] Grow bars
            (for _index (range (`KismetArrayLibrary.Array_Length` (`self.DataValues`)))
              (bind _returnvalue (`DataTableFunctionLibrary.GetDataTableColumnAsString` "/Game/Team_statistics/Game_Statistics.Game_Statistics" "TeamH"))
              (bind _returnvalue_2 (`DataTableFunctionLibrary.GetDataTableColumnAsString` "/Game/Team_statistics/Game_Statistics.Game_Statistics" "TeamA"))
              (bind _output (`|GetArrayItem` _returnvalue _index))
              (bind _output_2 (`|GetArrayItem` _returnvalue_2 _index))
              (if (> (`KismetStringLibrary.Conv_StringToDouble` _output) (`KismetStringLibrary.Conv_StringToDouble` _output_2))
                (set `self.Higher value` _output)
                (else
                  (set `self.Higher value` _output_2)))
              (`self.UpdateData` (`|GetArrayItem` (`self.AMesh`) _index) (`|GetArrayItem` (`self.AText`) _index) (* _growfactor (`|GetArrayItem` (`self.DataValues`) _index)) (* _size_y 2.0) (`self.Higher value`))))
          (:`Finished`
            (bind _returnvalue_3 (xor _isa (not _initatzero)))
            (if _returnvalue_3
              (bind (_direction_2 _fadefactor) (`Timeline|FadeTimeline` :!via `PlayFromStart` :!label _label_3)
                (:`Update`
                  ;[1 1 1] Fade Text
                  (for _array_element (`self.AText`)
                    (`self.SetTextOpacity` _array_element _fadefactor)))
                (:`Finished`
                  (if (not _returnvalue_3)
                    (goto _label_2 :!via `ReverseFromEnd`))))
              (else
                (`SceneComponent.SetVisibility` _defaultsceneroot false true)))))
        (else
          (goto _label_3 :!via `ReverseFromEnd`))))
    (:`B`
      (if _initatzero
        (goto _label_3 :!via `ReverseFromEnd`)
        (else
          (goto _label))))))

(fn `UpdateData`
  (params (Mesh :type "StaticMeshComponent Object Reference") (Text :type "TextRenderComponent Object Reference") (Value :type "Float (double-precision)") (Scale :type "Float (double-precision)") (Higher :type String))
  (locals (`Max Data Value` :type "Float (double-precision)"))
  (bind (_relativelocation_x _relativelocation_y) (`KismetMathLibrary.BreakVector` (`SceneComponent.RelativeLocation` Mesh)))
  (bind (_textoffset_x _textoffset_y) (`KismetMathLibrary.BreakVector2D` (`self.TextOffset`)))
  (bind (_returnvalue_x _returnvalue_y _returnvalue_z) (`KismetMathLibrary.BreakVector` (`SceneComponent.K2_GetComponentScale` (`self.DefaultSceneRoot`))))
  (bind _returnvalue (* Scale (/ Value (`KismetStringLibrary.Conv_StringToDouble` Higher))))
  (`MeshComponent.SetVectorParameterValueOnMaterials` Mesh "Color" (`self.VecCurveValue` Value))
  (`SceneComponent.SetWorldScale3D` Mesh (`KismetMathLibrary.MakeVector` _returnvalue_x _returnvalue_y (* _returnvalue_z _returnvalue)))
  (`TextRenderComponent.K2_SetText` Text (`KismetTextLibrary.Conv_IntToText` (`KismetMathLibrary.FTrunc` Value)))
  (`PrimitiveComponent.SetCullDistance` Text 0.0)
  (`SceneComponent.K2_SetRelativeLocation` Text (`KismetMathLibrary.MakeVector` (+ _relativelocation_x _textoffset_x) _relativelocation_y (+ (* _returnvalue 10.0) _textoffset_y)) false false)
  (return))

(fn `UserConstructionScript`
  (bind (_textoffset_x _textoffset_y) (`KismetMathLibrary.BreakVector2D` (`self.TextOffset`)))
  (bind _fadetimeline (`self.FadeTimeline`))
  (bind _fadecurve (`self.FadeCurve`))
  (bind _growtimeline (`self.GrowTimeline`))
  (bind _growcurve (`self.GrowCurve`))
  (bind _size_x (`KismetMathLibrary.BreakVector2D` (`self.Size`)))
  (bind (_size_x_2 _size_y) (`KismetMathLibrary.BreakVector2D` (`self.Size`)))
  (`parent.UserConstructionScript`)
  (`|ExecutionSequence`
    (:`then_0`
      (`TimelineComponent.SetFloatCurve` _fadetimeline _fadecurve "FadeFactor")
      (`TimelineComponent.SetTimelineLength` _fadetimeline (`.MaxTime` (`CurveBase.GetTimeRange` _fadecurve)))
      (`TimelineComponent.SetFloatCurve` _growtimeline _growcurve "GrowFactor")
      (`TimelineComponent.SetTimelineLength` _growtimeline (`.MaxTime` (`CurveBase.GetTimeRange` _growcurve))))
    (:`then_1`
      (for _index (range (`KismetArrayLibrary.Array_Length` (`self.DataValues`)))
        (`|ExecutionSequence`
          (:`then_0`
            (bind _returnvalue (* _index _size_x))
            (bind _textrender (`self.CreateTextComponent` 0.0 (`KismetMathLibrary.MakeTransform` (`KismetMathLibrary.MakeVector` (+ _textoffset_x _returnvalue) 0.0 _textoffset_y) (`KismetMathLibrary.MakeRotator` 90.0 (`self.TextRotation`) 90.0)) (select `bool` (`self.InitAtZero`) :`false` 1.0))))
          (:`then_1`
            (bind _returnvalue_2 (`self.CreateMeshComp` (`KismetMathLibrary.MakeTransform` (`KismetMathLibrary.MakeVector` _returnvalue))))
            (`KismetArrayLibrary.Array_Add` (`self.AMesh`) _returnvalue_2))
          (:`then_2`
            (`self.UpdateData` _returnvalue_2 _textrender (select `bool` (`self.InitAtZero`) :`false` (`|GetArrayItem` (`self.DataValues`) _index) :`true` 0.01) _size_y))))
      (`SceneComponent.SetVisibility` (`self.DefaultSceneRoot`) (not (`self.InitAtZero`)) true))))