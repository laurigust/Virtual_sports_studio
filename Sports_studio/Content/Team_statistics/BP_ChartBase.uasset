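; Base actor for data-driven statistics charts, leaving BuildChart empty for child classes to implement.
; The construction script reads a DataTable column as strings, keeps numeric entries, caches their maximum, and hides the root hierarchy when InitAtZero is set.
; Helpers spawn styled text labels with opacity set through color alpha, and map values normalized by that maximum to colors from the ColorMap curve.
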(event `BuildChart`)

(fn `Build Chart`)

(fn `CreateTextComponent`
  (params (DataValue :type "Float (double-precision)") (RelativeTransformation :type "Transform Structure") (Opacity :type "Float (double-precision)"))
  (returns (TextRender :type "TextRenderComponent Object Reference"))
  (bind _returnvalue (`AddComponent|NODE_AddTextRenderComponent-0` :`RelativeTransform` RelativeTransformation))
  (`|ExecutionSequence`
    (:`then_0`
      (`TextRenderComponent.K2_SetText` _returnvalue (`KismetTextLibrary.Conv_DoubleToText` DataValue "HalfToEven" false true 1 324 2 2)))
    (:`then_1`
      (`TextRenderComponent.SetFont` _returnvalue (`self.Font`)))
    (:`then_2`
      (`TextRenderComponent.SetWorldSize` _returnvalue (`self.FontSize`)))
    (:`then_3`
      (`TextRenderComponent.SetTextRenderColor` _returnvalue (`self.FontColor`)))
    (:`then_4`
      (`KismetArrayLibrary.Array_Add` (`self.AText`) _returnvalue))
    (:`then_5`
      (`self.SetTextOpacity` _returnvalue Opacity))
    (:`then_6`
      (return _returnvalue))))

(fn `SetTextOpacity`
  (params (TextRenderComponent :type "TextRenderComponent Object Reference") (Alpha :type "Float (double-precision)"))
  (bind (_b _g _r) (break `Color` (`TextRenderComponent.TextRenderColor` TextRenderComponent)))
  (`TextRenderComponent.SetTextRenderColor` TextRenderComponent (make `Color` _b _g _r (`KismetMathLibrary.Conv_IntToByte` (`KismetMathLibrary.FTrunc` (* Alpha 255.0))))))

(fn `UserConstructionScript`
  (`|ExecutionSequence`
    (:`then_0`
      (`KismetArrayLibrary.Array_Clear` (`self.DataValues`))
      (bind _returnvalue (`DataTableFunctionLibrary.GetDataTableColumnAsString` (`self.DataTable`) (`self.ColumnName`)))
      (for _array_element _returnvalue
        (if (`KismetStringLibrary.IsNumeric` _array_element)
          (`KismetArrayLibrary.Array_Add` (`self.DataValues`) (`KismetStringLibrary.Conv_StringToDouble` _array_element)))))
    (:`then_1`
      (set `self.MaxDataValue` (`.MaxValue` (`KismetMathLibrary.MaxOfFloatArray` (`self.DataValues`))))
      (`SceneComponent.SetVisibility` (`self.DefaultSceneRoot`) (not (`self.InitAtZero`)) true))))

(fn `VecCurveValue`
  (params (Value :type "Float (double-precision)"))
  (returns (VecColor :type "Vector Structure"))
  (return (`KismetMathLibrary.Conv_LinearColorToVector` (`CurveLinearColor.GetLinearColorValue` (`self.ColorMap`) (/ Value (`self.MaxDataValue`))))))