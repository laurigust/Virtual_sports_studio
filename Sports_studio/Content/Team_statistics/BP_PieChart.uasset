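; Animated 3D pie chart actor that renders DataValues as procedural mesh slices, with angle set by share and height by value.
; The construction script creates one GenerateSlice section per value, with a ColorMap-tinted dynamic material and a text label.
; BuildChart toggles show and hide via FlipFlop, with InitAtZero setting the starting state.
; Curve-driven timelines sweep slices open by updating vertices, then fade labels in, reversing to hide.
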(event `self.BuildChart`
  (bind (_size_x _size_y) (`KismetMathLibrary.BreakVector2D` (`self.Size`)))
  (bind _proceduralmesh (`self.ProceduralMesh`))
  (bind _angles (`self.angles`))
  (bind _initatzero (`self.InitAtZero`))
  ;[1 1 1] Combinations of 4 cases that call each other :(
  (bind _isa (`/Engine/EditorBlueprintResources/StandardMacros.FlipFlop`)
    (:`A`
      (if _initatzero
        (`SceneComponent.SetVisibility` _proceduralmesh true false :!label _label)
        (bind (_direction _growfactor) (`Timeline|GrowTimeline` :!via `PlayFromStart` :!label _label_2)
          (:`Update`
            ;[1 1 1] Grow Sections
            (for (_array_element _array_index) (`self.DataValues`)
              (bind _returnvalue (* _growfactor 360.0))
              (bind (_pos _tris _norms) (`self.GenerateSlice` (`KismetMathLibrary.FMin` _returnvalue (`|GetArrayItem` _angles _array_index)) (`KismetMathLibrary.FMin` _returnvalue (`|GetArrayItem` _angles (+ _array_index 1))) (`|GetArrayItem` (`self.sectionsubs`) _array_index) _size_x (* _array_element _size_y) (`self.Gap`)))
              (`ProceduralMeshComponent.UpdateMeshSection_LinearColor` :`self` (`self.ProceduralMesh`) :`SectionIndex` _array_index :`Vertices` _pos :`Normals` _norms)))
          (:`Finished`
            (bind _returnvalue_2 (xor _isa (not _initatzero)))
            (if _returnvalue_2
              (bind (_direction_2 _fadefactor) (`Timeline|FadeTimeline` :!via `PlayFromStart` :!label _label_3)
                (:`Update`
                  ;[1 1 1] Fade Text
                  (for _array_element_2 (`self.AText`)
                    (`self.SetTextOpacity` _array_element_2 _fadefactor)))
                (:`Finished`
                  (if (not _returnvalue_2)
                    (goto _label_2 :!via `ReverseFromEnd`))))
              (else
                (`SceneComponent.SetVisibility` _proceduralmesh false false)))))
        (else
          (goto _label_3 :!via `ReverseFromEnd`))))
    (:`B`
      (if _initatzero
        (goto _label_3 :!via `ReverseFromEnd`)
        (else
          (goto _label))))))

(fn `ArraySum`
  (params (Array :type "Array of Float (double-precision)"))
  (returns (Sum :type "Float (double-precision)"))
  (locals (Accum :type "Float (double-precision)"))
  (bind _accum (`local.Accum`))
  (for _array_element Array
    (set `local.Accum` (+ _array_element _accum)))
  (return _accum))

(fn `GenerateSlice`
  (params (AngleStart :type "Float (double-precision)") (AngleEnd :type "Float (double-precision)") (Subdivisions :type Integer) (Radius :type "Float (double-precision)") (Thickness :type "Float (double-precision)") (Offset :type "Float (double-precision)"))
  (returns (Pos :type "Array of Vector Structure") (Tris :type "Array of Integer") (Norms :type "Array of Vector Structure"))
  (locals (CapPos :type "Array of Vector Structure") (BasePos :type "Array of Vector Structure") (SidesPos :type "Array of Vector Structure") (SectionPos :type "Array of Vector Structure") (BaseNorms :type "Array of Vector Structure") (CapNorms :type "Array of Vector Structure") (SideNorms :type "Array of Vector Structure") (SectionNorms :type "Array of Vector Structure") (CapTris :type "Array of Integer") (BaseTris :type "Array of Integer") (SidesTris :type "Array of Integer") (SectionTris :type "Array of Integer") (lastvertid :type Integer))
  (bind _returnvalue (- Subdivisions 1))
  (bind _returnvalue_2 (+ AngleStart Offset))
  (bind (_x _y) (`self.GetHalfAngle` AngleStart AngleEnd))
  (bind _sidestris (`local.SidesTris`))
  (bind _basepos (`local.BasePos`))
  (bind _cappos (`local.CapPos`))
  (bind _sidespos (`local.SidesPos`))
  (bind _lastvertid (`local.lastvertid`))
  (bind _returnvalue_3 (`KismetArrayLibrary.Array_Length` (`local.SidesPos`)))
  (bind _returnvalue_4 (+ (`local.lastvertid`) 2))
  (bind _returnvalue_5 (/ _returnvalue_3 2))
  (`|ExecutionSequence`
    (:`then_0`
      (`KismetArrayLibrary.Array_Add` (`local.BasePos`) (`KismetMathLibrary.MakeVector` (* _x Offset) (* _y Offset)))
      (`KismetArrayLibrary.Array_Add` (`local.BaseNorms`) (0.0 0.0 -1.0))
      (for _index (range (+ _returnvalue 1))
        (bind _returnvalue_6 (+ _returnvalue_2 (* (/ (- (- AngleEnd Offset) _returnvalue_2) (`KismetMathLibrary.Conv_IntToDouble` _returnvalue)) (`KismetMathLibrary.Conv_IntToDouble` _index))))
        (`KismetArrayLibrary.Array_Add` (`local.BasePos`) (`KismetMathLibrary.MakeVector` (* (`KismetMathLibrary.DegSin` _returnvalue_6) Radius) (* (`KismetMathLibrary.DegCos` _returnvalue_6) Radius)))
        (`KismetArrayLibrary.Array_Add` (`local.BaseNorms`) (0.0 0.0 -1.0)))
      (set `local.lastvertid` (+ _index 1))
      (for _index_2 (range (+ (- (`KismetArrayLibrary.Array_Length` (`local.BasePos`)) 3) 1))
        (`self.AddTriangle` (+ _index_2 2) (+ _index_2 1) 0 (`local.BaseTris`))))
    (:`then_1`
      (for _array_element (`local.BasePos`)
        (`KismetArrayLibrary.Array_Add` (`local.CapPos`) (+ _array_element (`KismetMathLibrary.MakeVector` 0.0 0.0 Thickness)))
        (`KismetArrayLibrary.Array_Add` (`local.CapNorms`) (0.0 0.0 1.0)))
      (for _index_3 (range (+ (- (`KismetArrayLibrary.Array_Length` (`local.BasePos`)) 3) 1))
        (`self.AddTriangle` _lastvertid (+ _index_3 1 _lastvertid) (+ _index_3 2 _lastvertid) (`local.CapTris`)))
      (set `local.lastvertid` (+ _index_3 (`local.lastvertid`))))
    (:`then_2`
      (`|ExecutionSequence`
        (:`then_0`
          (`KismetArrayLibrary.Array_Append` (`local.SidesPos`) (`local.BasePos`))
          (`KismetArrayLibrary.Array_Append` (`local.SidesPos`) (`local.CapPos`))
          (`KismetArrayLibrary.Array_Remove` _sidespos)
          (`KismetArrayLibrary.Array_Remove` _sidespos (`KismetArrayLibrary.Array_LastIndex` (`local.BasePos`))))
        (:`then_1`
          (for _index_4 (range (+ (`KismetArrayLibrary.Array_LastIndex` (`local.SidesPos`)) 1))
            (bind _output (`|GetArrayItem` (`local.SidesPos`) _index_4))
            (`KismetArrayLibrary.Array_Add` (`local.SideNorms`) (`KismetMathLibrary.Normal` (- _output (* _output (0.0 0.0 1.0)))))))
        (:`then_2`
          (for _index_5 (range _returnvalue_4 (+ (- (+ _returnvalue_4 _returnvalue_5) 2) 1))
            (`|ExecutionSequence`
              (:`then_0`
                (bind _returnvalue_7 (+ _index_5 1))
                (bind _returnvalue_8 (+ _index_5 _returnvalue_5))
                (`self.AddTriangle` _index_5 _returnvalue_7 _returnvalue_8 _sidestris))
              (:`then_1`
                (`self.AddTriangle` (+ _returnvalue_8 1) _returnvalue_8 _returnvalue_7 _sidestris))))
          (set `local.lastvertid` (+ (`local.lastvertid`) _returnvalue_3 6)))
        (:`then_3`
          (`self.CreateSidePoly` (`local.SidesPos`) (`local.SideNorms`) (`local.SidesTris`) (`local.lastvertid`) (`local.BasePos`) (`local.CapPos`) 1 1)
          (bind _output_get (set `local.lastvertid` (+ (`local.lastvertid`) 4)))
          (`self.CreateSidePoly` (`local.SidesPos`) (`local.SideNorms`) (`local.SidesTris`) _output_get _basepos _cappos (`KismetArrayLibrary.Array_LastIndex` _basepos) (`KismetArrayLibrary.Array_LastIndex` _cappos) true))))
    (:`then_3`
      (`|ExecutionSequence`
        (:`then_0`
          (`self.MergeArrays` (`local.BasePos`) (`local.CapPos`) (`local.SidesPos`) (`local.SectionPos`))
          (`self.MergeArrays` (`local.BaseNorms`) (`local.CapNorms`) (`local.SideNorms`) (`local.SectionNorms`))
          (`self.MergeArrays` (`local.BaseTris`) (`local.CapTris`) (`local.SidesTris`) (`local.SectionTris`)))
        (:`then_1`
          (return (`local.SectionPos`) (`local.SectionTris`) (`local.SectionNorms`)))))))

(fn `UserConstructionScript`
  (bind (_size_x _size_y) (`KismetMathLibrary.BreakVector2D` (`self.Size`)))
  (bind _fadetimeline (`self.FadeTimeline`))
  (bind _datavalues (`self.DataValues`))
  (bind _fadecurve (`self.FadeCurve`))
  (bind _growtimeline (`self.GrowTimeline`))
  (bind _size_x_2 (`KismetMathLibrary.BreakVector2D` (`self.Size`)))
  (bind _growcurve (`self.GrowCurve`))
  (bind (_textoffset_x _textoffset_y) (`KismetMathLibrary.BreakVector2D` (`self.TextOffset`)))
  (bind _initatzero (`self.InitAtZero`))
  (bind _lastangle (`self.lastangle`))
  (bind _returnvalue (+ _size_x_2 _textoffset_x))
  (`parent.UserConstructionScript`)
  (`|ExecutionSequence`
    (:`then_0`
      (`TimelineComponent.SetFloatCurve` _fadetimeline _fadecurve "FadeFactor")
      (`TimelineComponent.SetTimelineLength` _fadetimeline (`.MaxTime` (`CurveBase.GetTimeRange` _fadecurve)))
      (`TimelineComponent.SetFloatCurve` _growtimeline _growcurve "GrowFactor")
      (`TimelineComponent.SetTimelineLength` _growtimeline (`.MaxTime` (`CurveBase.GetTimeRange` _growcurve)))
      (`KismetArrayLibrary.Array_Clear` (`self.angles`))
      (`KismetArrayLibrary.Array_Add` (`self.angles`))
      (`SceneComponent.SetVisibility` (`self.ProceduralMesh`) (not (`self.InitAtZero`)) false))
    (:`then_1`
      (set `self.lastangle` 0.0)
      (bind _sum (`self.ArraySum` _datavalues))
      (for (_array_element _array_index) _datavalues
        (bind _returnvalue_2 (/ _array_element _sum))
        (bind _returnvalue_3 (+ (* _returnvalue_2 360.0) (`self.lastangle`)))
        (`KismetArrayLibrary.Array_Add` (`self.angles`) _returnvalue_3)
        (bind _returnvalue_4 (`KismetMathLibrary.Max` (`KismetMathLibrary.FCeil` (* (`self.Subdivisions`) _returnvalue_2)) 2))
        (`KismetArrayLibrary.Array_Add` (`self.sectionsubs`) _returnvalue_4)
        (bind _returnvalue_5 (* _array_element _size_y))
        (bind (_pos _tris _norms) (`self.GenerateSlice` (select `bool` _initatzero :`false` _lastangle) (select `bool` _initatzero :`false` _returnvalue_3) _returnvalue_4 _size_x _returnvalue_5 (`self.Gap`)))
        (`ProceduralMeshComponent.CreateMeshSection_LinearColor` :`self` (`self.ProceduralMesh`) :`SectionIndex` _array_index :`Vertices` _pos :`Triangles` _tris :`Normals` _norms)
        (bind _returnvalue_6 (`PrimitiveComponent.CreateDynamicMaterialInstance` (`self.ProceduralMesh`) _array_index "/Game/Materials/M_Chart.M_Chart" "None"))
        (`MaterialInstanceDynamic.SetVectorParameterValue` _returnvalue_6 "Color" (`CurveLinearColor.GetLinearColorValue` (`self.ColorMap`) (/ _array_element (`self.MaxDataValue`))))
        (bind (_x _y) (`self.GetHalfAngle` _lastangle _returnvalue_3))
        (`self.CreateTextComponent` _array_element (`KismetMathLibrary.MakeTransform` (`KismetMathLibrary.MakeVector` (* _x _returnvalue) (* _y _returnvalue) (+ _returnvalue_5 _textoffset_y)) (`KismetMathLibrary.MakeRotator` (`self.TextRotation`) 90.0)) (select `bool` (`self.InitAtZero`) :`false` 1.0))
        (set `self.lastangle` _returnvalue_3)))))