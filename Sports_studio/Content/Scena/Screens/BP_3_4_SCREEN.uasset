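; Virtual-set 3:4 LED screen actor that displays an Aximmetry video feed and turns to face the Aximmetry camera.
; BeginPlay puts a dynamic LED3_4 material on the Screen component, and Tick pushes the "3on4 SCREEN INPUT" video into its texture parameter.
; Tick also smoothly interpolates the screen's yaw toward the Aximmetry camera transform with a quarter-turn offset, keeping pitch and roll unchanged.
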(event `self.ReceiveBeginPlay`
  (bind _screen (`self.Screen`))
  ;[1 1 1] set texture
  (bind _returnvalue (`PrimitiveComponent.CreateDynamicMaterialInstance` _screen 0 "/Game/Scena/Screens/LED3_4.LED3_4" "None"))
  (`PrimitiveComponent.SetMaterial` _screen 0 _returnvalue))

(event `self.ReceiveTick`
  (params (DeltaSeconds :type "Float (single-precision)"))
  (bind _returnvalue (`self.GetAximmetryTransformation` "CAMERA TRANFORM"))
  (bind _screen (`self.Screen`))
  (bind (_returnvalue_x _returnvalue_y _returnvalue_z) (`KismetMathLibrary.BreakVector` (`SceneComponent.K2_GetComponentLocation` _screen)))
  (bind (_returnvalue_roll _returnvalue_pitch _returnvalue_yaw) (`KismetMathLibrary.BreakRotator` (`SceneComponent.K2_GetComponentRotation` _screen)))
  (bind (_returnvalue_roll_2 _returnvalue_pitch_2 _returnvalue_yaw_2) (`KismetMathLibrary.BreakRotator` (`KismetMathLibrary.FindLookAtRotation` (`KismetMathLibrary.MakeVector` _returnvalue_x _returnvalue_y _returnvalue_z) (`KismetMathLibrary.MakeVector` (.x (.location _returnvalue)) (.y (.location _returnvalue)) (.z (.location _returnvalue))))))
  (bind (_returnvalue_roll_3 _returnvalue_pitch_3 _returnvalue_yaw_3) (`KismetMathLibrary.BreakRotator` (`KismetMathLibrary.RInterpTo` (`KismetMathLibrary.MakeRotator` _returnvalue_roll _returnvalue_pitch _returnvalue_yaw) (`KismetMathLibrary.MakeRotator` _returnvalue_pitch_2 _returnvalue_roll_2 (+ _returnvalue_yaw_2 90.0)) (`GameplayStatics.GetWorldDeltaSeconds`) 1.5)))
  (`|ExecutionSequence`
    (:`then_0`
      ;[1 1 1] set texture
      (bind _returnvalue_2 (`self.GetAximmetryVideo` "3on4 SCREEN INPUT"))
      (`MaterialInstanceDynamic.SetTextureParameterValue` (stale `self.ReceiveBeginPlay` _returnvalue) "LEDINPUT3_4" _returnvalue_2))
    (:`then_1`
      ;[1 1 1] Set rotation to camera
      (`SceneComponent.K2_SetWorldRotation` _screen (`KismetMathLibrary.MakeRotator` _returnvalue_roll _returnvalue_pitch _returnvalue_yaw_3) false false))))

(fn `UserConstructionScript`)